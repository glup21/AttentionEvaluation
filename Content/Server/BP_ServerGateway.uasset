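; BP_ServerGateway periodically uploads data from the player's first-person character to a local HTTP server.
; On BeginPlay it caches the controlled BP_FirstPersonCharacter and starts a looping timer that fires five times a second.
; Each tick converts the character's NewTimestamp struct to JSON and POSTs it to a localhost data endpoint, printing an error if the request fails.
; The response body is not used.
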(event Custom|SendDataToServer
  (bind (_outjsonstring _returnvalue) (|StructtoJsonString (Variables|/Game/FirstPerson/Blueprints/BP_FirstPersonCharacter.BP_FirstPersonCharacter_C|GetNewTimestamp (Variables|Default|GetAs%20BP%20First%20Person%20Character))))
  (if _returnvalue
    (bind _result_body (|HttpRequest :Url "http://localhost:3000/data" :Verb "Post" :Body _outjsonstring)
      (:On%20Error
        (Development|PrintString "Error connecting to a server!")))))

(event EventBeginPlay
  (bind _asbp_first_person_character (Utilities|Casting|CastToBP_FirstPersonCharacter (Pawn|GetControlledPawn (Game|GetPlayerController 0))))
  (Variables|Default|SetAs%20BP%20First%20Person%20Character _asbp_first_person_character)
  (Utilities|Time|SetTimerbyEvent (delegate Custom|SendDataToServer) 0.2 true true))

(fn ConstructionScript)